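; BP_GameMode runs a timed score round, creating the WBP_InGameHUD widget and printing a start message on BeginPlay.
; AddScore accumulates TotalScore and pushes it to the HUD.
; Tick uses a one-second Delay to throttle the TimeSeconds countdown while refreshing the timer text every frame.
; When time runs out, it prints an end message and restarts the level through the RestartLevel console command.
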(event Custom|AddScore
  (params (AddedScore :type Integer))
  ;[1 1 1] Add Score
  (bind _output_get (Variables|Default|SetTotalScore (+ AddedScore (Variables|Default|GetTotalScore))))
  (Default|UpdateScoreText (Variables|Default|GetInGameHUD) _output_get))

(event EventBeginPlay
  ;[1 1 1] コメント
  (Utilities|FlowControl|Sequence
    (:then_0
      ;;[1 1 1] 初級課題Startの表示
      (Variables|Default|SetStartTime (Math|DateTime|Now))
      (Development|PrintString "スタート！" true true "(R=0.000000,G=0.660000,B=1.000000,A=1.000000)" 5.0))
    (:then_1
      ;;[1 1 1] コメント
      (bind _returnvalue (UserInterface|CreateWidget "/Game/Hikanyan_Assets/UI/WBP_InGameHUD.WBP_InGameHUD_C"))
      (bind _output_get (Variables|Default|SetInGameHUD _returnvalue))
      (UserInterface|Viewport|AddtoViewport _output_get 0)
      (Default|UpdateScoreText (Variables|Default|GetInGameHUD) (Variables|Default|GetTotalScore))
      (Default|UpdateTimerText (Variables|Default|GetInGameHUD) 0.0))))

(event EventTick
  (params (DeltaSeconds :type Float%20%28single-precision%29))
  ;[1 1 1] Timer
  (Utilities|FlowControl|Sequence
    (:then_0
      (Utilities|FlowControl|Delay 1.0)
      (bind _result (Math|Float|DecrementFloat (Variables|Default|GetTimeSeconds))
        (:%20%20
          (if (not (> _result 0.0))
            (Development|PrintString "終了" true true "(R=0.892800,G=0.247920,B=1.000000,A=1.000000)" 5.0)
            (Development|ExecuteConsoleCommand "RestartLevel" 0)))))
    (:then_1
      (Default|UpdateTimerText (Variables|Default|GetInGameHUD) _result))))

(fn ConstructionScript)